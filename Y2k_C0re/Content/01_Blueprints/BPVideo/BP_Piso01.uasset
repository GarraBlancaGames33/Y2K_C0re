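; Floor trigger actor that opens a video when the player pawn steps into its Box and closes it when the player leaves.
; On BeginPlay it caches the BP_Video01 actor found in the level and the BP_ThirdPersonGameMode.
; Box overlap events call AbrirVideo or CerrarVideo on the video actor and notify the game mode through Entrar or Salir.
; Its own Entrar function is an empty stub.
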(event `self.ReceiveBeginPlay`
  (`|ExecutionSequence`
    (:`then_0`
      (bind _returnvalue (`GameplayStatics.GetActorOfClass` "/Game/01_Blueprints/BPVideo/BP_Video01.BP_Video01_C"))
      (set `self.BPVideo` _returnvalue))
    (:`then_1`
      (bind _asbp_third_person_game_mode (cast `/Game/01_Blueprints/Personaje/BP_ThirdPersonGameMode` (`GameplayStatics.GetGameMode`)))
      (set `self.As BP Third Person Game Mode` _asbp_third_person_game_mode))))

(event `self.Box.OnComponentBeginOverlap`
  (params (OverlappedComponent :type "PrimitiveComponent Object Reference") (OtherActor :type "Actor Object Reference") (OtherComp :type "PrimitiveComponent Object Reference") (OtherBodyIndex :type Integer) (bFromSweep :type Boolean) (SweepResult :type "HitResult Structure (by ref)"))
  (if (== OtherActor (`GameplayStatics.GetPlayerPawn` 0))
    (`/Game/01_Blueprints/BPVideo/BP_Video01.AbrirVideo` (`self.BPVideo`))
    (`/Game/01_Blueprints/Personaje/BP_ThirdPersonGameMode.Entrar` (`self.As BP Third Person Game Mode`))))

(event `self.Box.OnComponentEndOverlap`
  (params (OverlappedComponent :type "PrimitiveComponent Object Reference") (OtherActor :type "Actor Object Reference") (OtherComp :type "PrimitiveComponent Object Reference") (OtherBodyIndex :type Integer))
  (if (== OtherActor (`GameplayStatics.GetPlayerPawn` 0))
    (`/Game/01_Blueprints/BPVideo/BP_Video01.CerrarVideo` (`self.BPVideo`))
    (`/Game/01_Blueprints/Personaje/BP_ThirdPersonGameMode.Salir` (`self.As BP Third Person Game Mode`))))

(fn `Entrar`)

(fn `UserConstructionScript`)