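; TV Blueprint that switches channel videos based on hex codes read from an Arduino over a serial COM port.
; BeginPlay opens the port and starts SerialReadLoop, while EndPlay closes it.
; The loop reads a line, compares it against nine hard-indexed DT_InfoCanales rows, and opens the matching video in MediaPlayer.
; It re-calls itself after a short delay, and matches also re-enter it directly, bypassing that delay.
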(event `self.ReceiveBeginPlay`
  (bind (_bopened _returnvalue) (`SerialCom.OpenComPort` 5 115200))
  (if _bopened
    (`KismetSystemLibrary.PrintString` "Open")
    (set `self.Arduino` _returnvalue)
    (`self.Serial Read Loop`)
    (else
      (`KismetSystemLibrary.PrintString` "lol"))))

(event `self.ReceiveEndPlay`
  (params (EndPlayReason :type "EEndPlayReason Enum" :default "Destroyed"))
  (bind _arduino (`self.Arduino`))
  (`/Engine/EditorBlueprintResources/StandardMacros.IsValid` _arduino
    (:`Is Valid`
      (`SerialCom.Close` _arduino))))

(event `Serial Read Loop`
  (bind _canalhex_datatable (break `DataTableRowHandle` (`self.CanalHEX`)))
  (bind _canalhex_datatable_2 (break `DataTableRowHandle` (`self.CanalHEX`)))
  (bind _canalhex_datatable_3 (break `DataTableRowHandle` (`self.CanalHEX`)))
  (bind _canalhex_datatable_4 (break `DataTableRowHandle` (`self.CanalHEX`)))
  (bind _canalhex_datatable_5 (break `DataTableRowHandle` (`self.CanalHEX`)))
  (bind _canalhex_datatable_6 (break `DataTableRowHandle` (`self.CanalHEX`)))
  (bind _canalhex_datatable_7 (break `DataTableRowHandle` (`self.CanalHEX`)))
  (bind _canalhex_datatable_8 (break `DataTableRowHandle` (`self.CanalHEX`)))
  (bind _canalhex_datatable_9 (break `DataTableRowHandle` (`self.CanalHEX`)))
  (`|ExecutionSequence`
    (:`then_0`
      (bind (_bsuccess _returnvalue) (`SerialCom.Readln` (`self.Arduino`)))
      (bind _output_get (set `self.HEX` _returnvalue))
      (`KismetSystemLibrary.PrintString` _output_get)
      (`KismetSystemLibrary.Delay` 0.2)
      (`self.Serial Read Loop` :!label _label))
    (:`then_1`
      (bind _outrownames (`DataTableFunctionLibrary.GetDataTableRowNames` _canalhex_datatable))
      (bind _returnvalue_2 (`|GetDataTableRow` "/Game/01_Blueprints/Canales/DT_InfoCanales.DT_InfoCanales" (`|GetArrayItem` _outrownames))
        (:`then`
          (bind (_hex _video) (break `/Game/01_Blueprints/Canales/S_Canales` _returnvalue_2))
          (if (`KismetStringLibrary.EqualEqual_StrStr` _hex (`self.HEX`))
            (`MediaPlayer.OpenSource` (`self.Media Player`) _video)
            (goto _label)))))
    (:`then_2`
      (bind _outrownames_2 (`DataTableFunctionLibrary.GetDataTableRowNames` _canalhex_datatable_2))
      (bind _returnvalue_3 (`|GetDataTableRow` "/Game/01_Blueprints/Canales/DT_InfoCanales.DT_InfoCanales" (`|GetArrayItem` _outrownames_2 1))
        (:`then`
          (bind (_hex_2 _video_2) (break `/Game/01_Blueprints/Canales/S_Canales` _returnvalue_3))
          (if (`KismetStringLibrary.EqualEqual_StrStr` _hex_2 (`self.HEX`))
            (`MediaPlayer.OpenSource` (`self.Media Player`) _video_2)
            (goto _label)))))
    (:`then_3`
      (bind _outrownames_3 (`DataTableFunctionLibrary.GetDataTableRowNames` _canalhex_datatable_3))
      (bind _returnvalue_4 (`|GetDataTableRow` "/Game/01_Blueprints/Canales/DT_InfoCanales.DT_InfoCanales" (`|GetArrayItem` _outrownames_3 2))
        (:`then`
          (bind (_hex_3 _video_3) (break `/Game/01_Blueprints/Canales/S_Canales` _returnvalue_4))
          (if (`KismetStringLibrary.EqualEqual_StrStr` _hex_3 (`self.HEX`))
            (`MediaPlayer.OpenSource` (`self.Media Player`) _video_3)
            (goto _label)))))
    (:`then_4`
      (bind _outrownames_4 (`DataTableFunctionLibrary.GetDataTableRowNames` _canalhex_datatable_4))
      (bind _returnvalue_5 (`|GetDataTableRow` "/Game/01_Blueprints/Canales/DT_InfoCanales.DT_InfoCanales" (`|GetArrayItem` _outrownames_4 3))
        (:`then`
          (bind (_hex_4 _video_4) (break `/Game/01_Blueprints/Canales/S_Canales` _returnvalue_5))
          (if (`KismetStringLibrary.EqualEqual_StrStr` _hex_4 (`self.HEX`))
            (`MediaPlayer.OpenSource` (`self.Media Player`) _video_4)
            (goto _label)))))
    (:`then_5`
      (bind _outrownames_5 (`DataTableFunctionLibrary.GetDataTableRowNames` _canalhex_datatable_5))
      (bind _returnvalue_6 (`|GetDataTableRow` "/Game/01_Blueprints/Canales/DT_InfoCanales.DT_InfoCanales" (`|GetArrayItem` _outrownames_5 4))
        (:`then`
          (bind (_hex_5 _video_5) (break `/Game/01_Blueprints/Canales/S_Canales` _returnvalue_6))
          (if (`KismetStringLibrary.EqualEqual_StrStr` _hex_5 (`self.HEX`))
            (`MediaPlayer.OpenSource` (`self.Media Player`) _video_5)
            (goto _label)))))
    (:`then_6`
      (bind _outrownames_6 (`DataTableFunctionLibrary.GetDataTableRowNames` _canalhex_datatable_6))
      (bind _returnvalue_7 (`|GetDataTableRow` "/Game/01_Blueprints/Canales/DT_InfoCanales.DT_InfoCanales" (`|GetArrayItem` _outrownames_6 5))
        (:`then`
          (bind (_hex_6 _video_6) (break `/Game/01_Blueprints/Canales/S_Canales` _returnvalue_7))
          (if (`KismetStringLibrary.EqualEqual_StrStr` _hex_6 (`self.HEX`))
            (`MediaPlayer.OpenSource` (`self.Media Player`) _video_6)
            (goto _label)))))
    (:`then_7`
      (bind _outrownames_7 (`DataTableFunctionLibrary.GetDataTableRowNames` _canalhex_datatable_7))
      (bind _returnvalue_8 (`|GetDataTableRow` "/Game/01_Blueprints/Canales/DT_InfoCanales.DT_InfoCanales" (`|GetArrayItem` _outrownames_7 6))
        (:`then`
          (bind (_hex_7 _video_7) (break `/Game/01_Blueprints/Canales/S_Canales` _returnvalue_8))
          (if (`KismetStringLibrary.EqualEqual_StrStr` _hex_7 (`self.HEX`))
            (`MediaPlayer.OpenSource` (`self.Media Player`) _video_7)
            (goto _label)))))
    (:`then_8`
      (bind _outrownames_8 (`DataTableFunctionLibrary.GetDataTableRowNames` _canalhex_datatable_8))
      (bind _returnvalue_9 (`|GetDataTableRow` "/Game/01_Blueprints/Canales/DT_InfoCanales.DT_InfoCanales" (`|GetArrayItem` _outrownames_8 7))
        (:`then`
          (bind (_hex_8 _video_8) (break `/Game/01_Blueprints/Canales/S_Canales` _returnvalue_9))
          (if (`KismetStringLibrary.EqualEqual_StrStr` _hex_8 (`self.HEX`))
            (`MediaPlayer.OpenSource` (`self.Media Player`) _video_8)
            (goto _label)))))
    (:`then_9`
      (bind _outrownames_9 (`DataTableFunctionLibrary.GetDataTableRowNames` _canalhex_datatable_9))
      (bind _returnvalue_10 (`|GetDataTableRow` "/Game/01_Blueprints/Canales/DT_InfoCanales.DT_InfoCanales" (`|GetArrayItem` _outrownames_9 8))
        (:`then`
          (bind (_hex_9 _video_9) (break `/Game/01_Blueprints/Canales/S_Canales` _returnvalue_10))
          (if (`KismetStringLibrary.EqualEqual_StrStr` _hex_9 (`self.HEX`))
            (`MediaPlayer.OpenSource` (`self.Media Player`) _video_9)
            (goto _label)))))))

(fn `UserConstructionScript`)